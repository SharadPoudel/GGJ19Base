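; Car actor that drives along a given spline with an assigned mesh and destroys itself on reaching the last point.
; MoveCar starts the CarMovement timeline at an offset, with play rate inverse to Speed, mapping its alpha to spline distance for location and rotation.
; Each tick a debug-drawn line trace, offset along world +X, eases the play rate toward zero on a hit and restores it instantly when clear.
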(event `MoveCar`
  (params (SplineReference :type "/Game/Blueprint/Car/Spline Object Reference") (NewMesh :type "StaticMesh Object Reference") (Speed :type "Float (double-precision)"))
  (bind _currentspline (`self.CurrentSpline`))
  (bind _returnvalue (`KismetMathLibrary.Lerp` 0.0 (`SplineComponent.GetSplineLength` _currentspline) (`self.Alpha`)))
  (bind _output_get (set `self.Speed` Speed))
  (set `self.OriginalSpeed` _output_get)
  (set `self.CurrentSpline` (`/Game/Blueprint/Car/Spline.ChosenSpline` SplineReference))
  (`KismetArrayLibrary.Array_Shuffle` (`self.Cars`))
  (`StaticMeshComponent.SetStaticMesh` (`self.Car`) NewMesh)
  (`TimelineComponent.SetPlayRate` (`self.CarMovement`) (/ 1.0 Speed))
  (`TimelineComponent.SetNewTime` (`self.CarMovement`) (`self.StartOffset`))
  (bind (_direction _alpha) (`Timeline|CarMovement`)
    (:`Update`
      (set `self.Alpha` _alpha)
      (`self.K2_SetActorLocationAndRotation` (`SplineComponent.GetLocationAtDistanceAlongSpline` _currentspline _returnvalue "World") (`SplineComponent.GetRotationAtDistanceAlongSpline` _currentspline _returnvalue "World"))
      (if (== (`self.K2_GetActorLocation`) (`SplineComponent.GetLocationAtSplinePoint` _currentspline (- (`SplineComponent.GetNumberOfSplinePoints` (`self.CurrentSpline`)) 1) "World"))
        (`self.K2_DestroyActor`)))))

(event `self.ReceiveTick`
  (params (DeltaSeconds :type "Float (single-precision)"))
  (bind _currentspline (`self.CurrentSpline`))
  (bind _carmovement (`self.CarMovement`))
  (bind _returnvalue (`SplineComponent.GetLocationAtDistanceAlongSpline` _currentspline (`KismetMathLibrary.Lerp` 0.0 (`SplineComponent.GetSplineLength` _currentspline) (`self.Alpha`)) "World"))
  (bind (_outhit _returnvalue_2) (`KismetSystemLibrary.LineTraceSingle` :`Start` (+ _returnvalue (200.0 0.0 70.0)) :`End` (+ _returnvalue (900.0 0.0 70.0)) :`TraceChannel` "TraceTypeQuery1" :`DrawDebugType` "Persistent"))
  (if _returnvalue_2
    (bind _output_get (set `self.Speed` 0.0))
    (bind _output_get_2 (set `self.SmoothVelocity` (`KismetMathLibrary.FClamp` (+ (* DeltaSeconds (`self.SpeedSmooth`)) (`self.SmoothVelocity`)))))
    (`TimelineComponent.SetPlayRate` _carmovement (`KismetMathLibrary.Lerp` (/ 1.0 (`self.OriginalSpeed`)) _output_get _output_get_2))
    (if (not _returnvalue_2)
      (`/Engine/EditorBlueprintResources/StandardMacros.DoOnce` false :!label _label
        (:`Completed`
          (`TimelineComponent.SetPlayRate` _carmovement (`KismetMathLibrary.Lerp` 0.0 (/ 1.0 (`self.OriginalSpeed`))))
          (`KismetSystemLibrary.Delay` 1.0)
          (goto _label :!via `Reset`))))
    (else
      (`TimelineComponent.SetPlayRate` _carmovement (/ 1.0 (`self.OriginalSpeed`))))))

(fn `UserConstructionScript`)