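; Spline actor in the car folder that picks which of four splines is followed next, without repeats until all are used.
; BeginPlay gathers the splines into a working array and saves a copy as the original set.
; RandomSpline refills the working array from that copy when empty, shuffles it, stores the first entry as ChosenSpline and removes it from the pool.
; The actual spline following happens outside this Blueprint.
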(event `self.ReceiveBeginPlay`
  (bind _splinearray (`self.SplineArray`))
  (for _array_element (`|MakeArray` (`self.Spline`) (`self.Spline1`) (`self.Spline2`) (`self.Spline3`))
    (`KismetArrayLibrary.Array_Add` _splinearray _array_element)
    (set `self.OriginalSplineArray` _splinearray)))

(event `RandomSpline`
  (bind _splinearray (`self.SplineArray`))
  ;[1 1 1] Check if array is empty, if yes refill it
  (if (== (`KismetArrayLibrary.Array_Length` (`self.SplineArray`)) 0)
    (set `self.SplineArray` (`self.OriginalSplineArray`)))
  ;[1 1 1] Shuffles array and sets the chosen spline to follow
  (`KismetArrayLibrary.Array_Shuffle` _splinearray)
  (bind _output_get (set `self.ChosenSpline` (`|GetArrayItem` _splinearray)))
  (for _array_element _splinearray
    (if (== _array_element _output_get)
      (`KismetArrayLibrary.Array_RemoveItem` _splinearray _array_element))))

(fn `UserConstructionScript`)