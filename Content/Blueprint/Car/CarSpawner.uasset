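; Car spawner actor that periodically spawns moving cars along randomly chosen spline paths.
; BeginPlay caches the car mesh list and starts a looping SpawnCar timer, whose random interval is rolled only once.
; Each SpawnCar call randomizes the referenced spline, spawns a car actor, and hands it the spline, mesh and random speed.
; Meshes are drawn from a shuffled pool without replacement, refilled from the cached list when empty.
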(event `self.ReceiveBeginPlay`
  ;[1 1 1] Spawn Car
  (set `self.OriginalCars` (`self.Cars`))
  (`KismetSystemLibrary.K2_SetTimer` null "SpawnCar" (`KismetMathLibrary.RandomFloatInRange` (`self.MinTimerSpawn`) (`self.MaxTimerSpawn`)) true))

(event `self.ReceiveTick`
  (params (DeltaSeconds :type "Float (single-precision)"))
  ;[1 1 1] Not using
)

(fn `SpawnCar`
  (bind _cars (`self.Cars`))
  (bind _cars_2 (`self.Cars`))
  ;[1 1 1] Spawn car in random spline
  (`/Game/Blueprint/Car/Spline.RandomSpline` (`self.SplineRef`))
  (bind _returnvalue (`|SpawnActorFromClass` "/Game/Blueprint/Car/CarBP.CarBP_C" (`self.GetTransform`) "AdjustIfPossibleButDontSpawnIfColliding" "OverrideRootScale" null null))
  ;[1 1 1] Check if array is empty, if yes refills it
  (if (== (`KismetArrayLibrary.Array_Length` _cars) 0)
    (set `self.Cars` (`self.OriginalCars`)))
  (`KismetArrayLibrary.Array_Shuffle` _cars)
  (for (_array_element _array_index) _cars_2
    (if (== _array_index 0)
      (`/Game/Blueprint/Car/CarBP.MoveCar` _returnvalue (`self.SplineRef`) _array_element (`KismetMathLibrary.RandomFloatInRange` (`self.MinSpeed`) (`self.MaxSpeed`)))
      (`KismetArrayLibrary.Array_Remove` _cars_2)
      (break))))

(fn `UserConstructionScript`)