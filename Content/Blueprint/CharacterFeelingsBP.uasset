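; Character needs Blueprint that tracks Hunger, Energy and Social values, with refill and loss events for other classes to call.
; Looping named timers start on BeginPlay to drain Hunger and Social, stopping with a debug message at zero.
; Refills clamp to each maximum and restart stopped timers.
; Energy has no timer, and LoseEnergy subtracts current Energy from the amount passed in, the reverse of LoseHunger.
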(event `self.ReceiveBeginPlay`
  ;[1 1 1] Start every timer (overriden)
  (`self.HungerActivateTimer`)
  (`self.SocialActivateTimer`))

(event `RefillEnergy`
  (params (EnergyValue :type "Float (double-precision)"))
  ;[1 1 1] Energy
  ;;[1 1 1] Refill energy from another class
  (set `self.Energy` (`KismetMathLibrary.FClamp` (+ EnergyValue (`self.Energy`)) 0.0 (`self.MaxEnergy`))))

(event `RefillSocial`
  (params (SocialValue :type "Float (double-precision)"))
  ;[1 1 1] Social
  ;;[1 1 1] Refill social by hanging out
  (set `self.Social` (`KismetMathLibrary.FClamp` (+ SocialValue (`self.Social`)) 0.0 (`self.MaxSocial`)))
  (if (not (`KismetSystemLibrary.K2_IsTimerActive` null "SocialFunction"))
    (`KismetSystemLibrary.K2_SetTimer` null "SocialFunction" (`self.TimerSocial`) true)))

(event `RefillHunger`
  (params (FoodValue :type "Float (double-precision)"))
  ;[1 1 1] Hunger
  ;;[1 1 1] Refill hunger from another class (food)
  (set `self.Hunger` (`KismetMathLibrary.FClamp` (+ FoodValue (`self.Hunger`)) 0.0 (`self.MaxHunger`)))
  (if (not (`KismetSystemLibrary.K2_IsTimerActive` null "Hungering"))
    (`KismetSystemLibrary.K2_SetTimer` null "Hungering" (`self.TimerHunger`) true)))

(event `LoseHunger`
  (params (SubtractingHunger :type "Float (double-precision)"))
  ;[1 1 1] Hunger
  ;;[1 1 1] Call when something happens that can cause hunger to get worse
  (bind _output_get (set `self.Hunger` (`KismetMathLibrary.FMax` (- (`self.Hunger`) SubtractingHunger))))
  (`self.StopHungerTimer` _output_get "Hungering"))

(event `LoseEnergy`
  (params (SubtractingEnergy :type "Float (double-precision)"))
  ;[1 1 1] Energy
  ;;[1 1 1] Call when uses energy
  (set `self.Energy` (`KismetMathLibrary.FMax` (- SubtractingEnergy (`self.Energy`)))))

(event `SocialActivateTimer`
  ;[1 1 1] Social
  ;;[1 1 1] Social over time
  (`KismetSystemLibrary.K2_SetTimer` null "SocialFunction" (`self.TimerSocial`) true))

(event `HungerActivateTimer`
  ;[1 1 1] Hunger
  ;;[1 1 1] Hunger over time
  (`KismetSystemLibrary.K2_SetTimer` null "Hungering" (`self.TimerHunger`) true))

(fn `Hungering`
  (bind _output_get (set `self.Hunger` (`KismetMathLibrary.FMax` (- (`self.Hunger`) (`self.HungerValue`)))))
  (`self.StopHungerTimer` _output_get "Hungering"))

(fn `SocialFunction`
  (bind _output_get (set `self.Social` (`KismetMathLibrary.FMax` (- (`self.Social`) (`self.SocialValue`)))))
  (`self.StopSocialTimer` _output_get "SocialFunction"))

(fn `UserConstructionScript`)